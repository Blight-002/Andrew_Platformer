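; Boss enemy Blueprint for the platformer that continuously spawns chaser minions.
; On BeginPlay it calls SpawnChasers, which spawns a BP_Enemy_Chaser at each of four Scene component transforms.
; The event then waits TimeBetweenSpawns and calls itself again, forming an endless timed wave loop with no cap or stop condition.
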(event `SpawnChasers`
  (`|SpawnActorFromClass` "/Game/_Platformer/Blueprints/BP_Enemy_Chaser.BP_Enemy_Chaser_C" (`SceneComponent.GetSocketTransform` (`self.Scene`) "None" "RTS_World") "Undefined" "MultiplyWithRoot" null null)
  (`|SpawnActorFromClass` "/Game/_Platformer/Blueprints/BP_Enemy_Chaser.BP_Enemy_Chaser_C" (`SceneComponent.GetSocketTransform` (`self.Scene1`) "None" "RTS_World") "Undefined" "MultiplyWithRoot" null null)
  (`|SpawnActorFromClass` "/Game/_Platformer/Blueprints/BP_Enemy_Chaser.BP_Enemy_Chaser_C" (`SceneComponent.GetSocketTransform` (`self.Scene2`) "None" "RTS_World") "Undefined" "MultiplyWithRoot" null null)
  (`|SpawnActorFromClass` "/Game/_Platformer/Blueprints/BP_Enemy_Chaser.BP_Enemy_Chaser_C" (`SceneComponent.GetSocketTransform` (`self.Scene3`) "None" "RTS_World") "Undefined" "MultiplyWithRoot" null null)
  (`KismetSystemLibrary.Delay` (`self.TimeBetweenSpawns`))
  (`self.SpawnChasers`))

(event `self.ReceiveBeginPlay`
  (`parent.ReceiveBeginPlay`)
  (`self.SpawnChasers`))

(fn `UserConstructionScript`
  (`parent.UserConstructionScript`))