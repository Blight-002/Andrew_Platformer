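; BP_Platform_Vanishing is a platformer platform that vanishes after the player stands on it too long, then reappears.
; A trigger zone flags player pawn overlap, and Tick accumulates time while flagged, resetting it otherwise.
; At the lifetime limit it hides the actor and disables collision.
; After a delay, ReturnToDefault restores visibility, collision and the root transform saved at BeginPlay.
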(event `self.ReceiveBeginPlay`
  ;[0.1577 0.3696 0.4896 0.5] Set Start Position
  (set `self.StartTransform` (`self.GetTransform`)))

(event `self.ReceiveTick`
  (params (DeltaSeconds :type "Float (single-precision)"))
  ;[0.08767 0.5304 0.02362 0.5] Count Time On Platform
  (if (`self.IsPlayerOnPlatform`)
    (bind _output_get (set `self.TimeOnPlatform` (+ DeltaSeconds (`self.TimeOnPlatform`))))
    ;[0.01303 0.1354 0.000202 0.5] Hide Platform If lifespan reached
    (if (>= _output_get (`self.PlatformLifetime`))
      (`self.SetActorHiddenInGame` true)
      (`self.SetActorEnableCollision` false)
      ; Reapear after delay
      (`KismetSystemLibrary.Delay` (`self.TimeInvisible`))
      (`self.ReturnToDefault`))
    (else
      (set `self.TimeOnPlatform` 0.0))))

(event `self.PlatformTriggerZone.OnComponentBeginOverlap`
  (params (OverlappedComponent :type "PrimitiveComponent Object Reference") (OtherActor :type "Actor Object Reference") (OtherComp :type "PrimitiveComponent Object Reference") (OtherBodyIndex :type Integer) (bFromSweep :type Boolean) (SweepResult :type "HitResult Structure (by ref)"))
  ;[0.4375 0.1253 0.1253 0.5] Collider Check
  (if (== OtherActor (`GameplayStatics.GetPlayerPawn` 0))
    (set `self.IsPlayerOnPlatform` true)))

(event `self.PlatformTriggerZone.OnComponentEndOverlap`
  (params (OverlappedComponent :type "PrimitiveComponent Object Reference") (OtherActor :type "Actor Object Reference") (OtherComp :type "PrimitiveComponent Object Reference") (OtherBodyIndex :type Integer))
  ;[0.4375 0.1253 0.1253 0.5] Collider Check
  (if (== (`GameplayStatics.GetPlayerPawn` 0) OtherActor)
    (set `self.IsPlayerOnPlatform` false)))

(event `ReturnToDefault`
  ;[1 0 0 0.5] Return to Start
  (`SceneComponent.K2_SetWorldTransform` (`self.DefaultSceneRoot`) (`self.StartTransform`) false true)
  (set `self.TimeOnPlatform` 0.0)
  (`self.SetActorHiddenInGame` false)
  (`self.SetActorEnableCollision` true))

(fn `UserConstructionScript`)