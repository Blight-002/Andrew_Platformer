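; BP_Platform_Warping is a platformer actor that teleports the player to its TeleportPoint component after they leave its Box trigger.
; On end overlap, a FlipFlop acts on every other unblocked exit, waiting TimeUntilTeleport before moving the player pawn without sweep.
; InTempTime blocks retriggers during the delay, but is set before the player check and stays set if another actor triggers that branch.
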(event `self.Box.OnComponentEndOverlap`
  (params (OverlappedComponent :type "PrimitiveComponent Object Reference") (OtherActor :type "Actor Object Reference") (OtherComp :type "PrimitiveComponent Object Reference") (OtherBodyIndex :type Integer))
  (bind _returnvalue (`GameplayStatics.GetPlayerPawn` 0))
  (if (not (`self.InTempTime`))
    (`/Engine/EditorBlueprintResources/StandardMacros.FlipFlop`
      (:`A`
        (set `self.InTempTime` true)
        (if (== OtherActor _returnvalue)
          (`KismetSystemLibrary.Delay` (`self.TimeUntilTeleport`))
          (`self.K2_SetActorLocation` _returnvalue (`SceneComponent.K2_GetComponentLocation` (`self.TeleportPoint`)) false true)
          (set `self.InTempTime` false))))))

(fn `UserConstructionScript`
  (`parent.UserConstructionScript`))