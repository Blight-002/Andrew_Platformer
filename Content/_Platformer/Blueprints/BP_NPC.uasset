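; Platformer NPC that shows a widget while the player is inside its trigger and can play timed dialogue lines.
; BeginPlay caches the player character, which the trigger overlap events check to toggle the widget.
; ResetDialogue restarts the sequence at the first line.
; UpdateDialogue writes each line into the player's dialogue string, re-calls itself after a fixed delay, and clears the string after the last line.
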(event `self.ReceiveBeginPlay`
  (bind _asbp_third_person_character (cast `/Game/_Platformer/Blueprints/BP_ThirdPersonCharacter` (`GameplayStatics.GetPlayerPawn` 0)))
  (set `self.PlayerReference` _asbp_third_person_character))

(event `self.Trigger.OnComponentBeginOverlap`
  (params (OverlappedComponent :type "PrimitiveComponent Object Reference") (OtherActor :type "Actor Object Reference") (OtherComp :type "PrimitiveComponent Object Reference") (OtherBodyIndex :type Integer) (bFromSweep :type Boolean) (SweepResult :type "HitResult Structure (by ref)"))
  (if (== OtherActor (`self.PlayerReference`))
    (`SceneComponent.SetVisibility` (`self.Widget`) true false)))

(event `self.Trigger.OnComponentEndOverlap`
  (params (OverlappedComponent :type "PrimitiveComponent Object Reference") (OtherActor :type "Actor Object Reference") (OtherComp :type "PrimitiveComponent Object Reference") (OtherBodyIndex :type Integer))
  (if (== OtherActor (`self.PlayerReference`))
    (`SceneComponent.SetVisibility` (`self.Widget`) false false)))

(event `UpdateDialogue`
  (bind _currectdialogueline (`self.CurrectDialogueLine`))
  ; Update Dialogue
  (set `/Game/_Platformer/Blueprints/BP_ThirdPersonCharacter.CurrentDialogString` (`|GetArrayItem` (`self.DialogueLines`) (`self.CurrectDialogueLine`)) (`self.PlayerReference`))
  (`/Engine/EditorBlueprintResources/StandardMacros.IncrementInt` _currectdialogueline
    (:`  `
      (`KismetSystemLibrary.Delay` 2.0)
      (if (!= _currectdialogueline (`KismetArrayLibrary.Array_Length` (`self.DialogueLines`)))
        (`self.UpdateDialogue`)
        (else
          (set `/Game/_Platformer/Blueprints/BP_ThirdPersonCharacter.CurrentDialogString` "" (`self.PlayerReference`)))))))

(event `ResetDialogue`
  ; Comment
  (set `self.CurrectDialogueLine` 0)
  (`self.UpdateDialogue`))

(fn `UserConstructionScript`)