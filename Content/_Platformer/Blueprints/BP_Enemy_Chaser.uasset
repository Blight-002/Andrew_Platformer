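; Platformer enemy that chases the third-person player, hurts them on contact and drops coins when killed.
; While the player is inside DetectionZone, Tick turns the enemy toward them and drives movement input their way.
; Overlapping HitZone launches the player and damages the enemy, spawning randomly scattered BP_Coins at zero health before it is destroyed.
; Capsule hits knock the player back using the enemy's scaled velocity and apply player damage.
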(event `self.ReceiveBeginPlay`
  (bind _asbp_third_person_character (cast `/Game/_Platformer/Blueprints/BP_ThirdPersonCharacter` (`GameplayStatics.GetPlayerPawn` 0)))
  (set `self.PlayerReference` _asbp_third_person_character))

(event `self.DetectionZone.OnComponentBeginOverlap`
  (params (OverlappedComponent :type "PrimitiveComponent Object Reference") (OtherActor :type "Actor Object Reference") (OtherComp :type "PrimitiveComponent Object Reference") (OtherBodyIndex :type Integer) (bFromSweep :type Boolean) (SweepResult :type "HitResult Structure (by ref)"))
  ; Check if Player In Detection Zone
  (if (== OtherActor (`self.PlayerReference`))
    (set `self.CanDetectPlayer` true)))

(event `self.DetectionZone.OnComponentEndOverlap`
  (params (OverlappedComponent :type "PrimitiveComponent Object Reference") (OtherActor :type "Actor Object Reference") (OtherComp :type "PrimitiveComponent Object Reference") (OtherBodyIndex :type Integer))
  ; Check if Player In Detection Zone
  (if (== OtherActor (`self.PlayerReference`))
    (set `self.CanDetectPlayer` false)))

(event `self.ReceiveTick`
  (params (DeltaSeconds :type "Float (single-precision)"))
  (bind (_returnvalue_x _returnvalue_y) (`KismetMathLibrary.BreakVector` (`self.K2_GetActorLocation`)))
  (bind (_returnvalue_x_2 _returnvalue_y_2) (`KismetMathLibrary.BreakVector` (`self.K2_GetActorLocation` (`self.PlayerReference`))))
  ; Enemy movement
  (if (`self.CanDetectPlayer`)
    (`|ExecutionSequence`
      (:`then_0`
        ;; Look at Player
        (`self.K2_SetActorRotation` (`KismetMathLibrary.FindLookAtRotation` (`KismetMathLibrary.MakeVector` _returnvalue_x _returnvalue_y) (`KismetMathLibrary.MakeVector` _returnvalue_x_2 _returnvalue_y_2))))
      (:`then_1`
        ;; Chase Player
        (`self.AddMovementInput` (`KismetMathLibrary.Normal` (- (`self.K2_GetActorLocation` (`self.PlayerReference`)) (`self.K2_GetActorLocation`))))))))

(event `self.HitZone.OnComponentBeginOverlap`
  (params (OverlappedComponent :type "PrimitiveComponent Object Reference") (OtherActor :type "Actor Object Reference") (OtherComp :type "PrimitiveComponent Object Reference") (OtherBodyIndex :type Integer) (bFromSweep :type Boolean) (SweepResult :type "HitResult Structure (by ref)"))
  (if (== OtherActor (`self.PlayerReference`))
    (`|ExecutionSequence`
      (:`then_0`
        ; Launch Player
        (`self.LaunchCharacter` (`self.PlayerReference`) (`self.Launch Directon`) false false))
      (:`then_1`
        ; Damage and kill Enemy
        (bind _output_get (set `self.Health` (- (`self.Health`) (`self.Enemy Damage`))))
        (if (<= _output_get 0)
          (`self.Loot and Destroy`))))))

(event `self.CapsuleComponent.OnComponentHit`
  (params (HitComponent :type "PrimitiveComponent Object Reference") (OtherActor :type "Actor Object Reference") (OtherComp :type "PrimitiveComponent Object Reference") (NormalImpulse :type "Vector Structure") (Hit :type "HitResult Structure (by ref)"))
  ; Player Knockback
  (if (== OtherActor (`self.PlayerReference`))
    (`self.LaunchCharacter` (`self.PlayerReference`) (* (`self.GetVelocity`) (`self.KickBackStreanth`)) false false)
    (`/Game/_Platformer/Blueprints/BP_ThirdPersonCharacter.DamagePlayer` (`self.PlayerReference`) (`self.PlayerDamage`))))

(event `Loot and Destroy`
  (bind _returnvalue (`self.GetTransform`))
  (bind _coinsdropped (`self.CoinsDropped`))
  (for _ (range (+ (`KismetMathLibrary.RandomIntegerInRange` (/ _coinsdropped 2) _coinsdropped) 1))
    (`|SpawnActorFromClass` "/Game/_Platformer/Blueprints/BP_Coin.BP_Coin_C" (`KismetMathLibrary.MakeTransform` (`KismetMathLibrary.MakeVector` (+ (.x (.location _returnvalue)) (`KismetMathLibrary.RandomFloatInRange` -200.0 200.0)) (+ (.y (.location _returnvalue)) (`KismetMathLibrary.RandomFloatInRange` -200.0 200.0)) (.z (.location _returnvalue))) (.rotation _returnvalue) (.scale _returnvalue)) "Undefined" "MultiplyWithRoot" null null))
  (`self.K2_DestroyActor`))

(fn `UserConstructionScript`)