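; Enemy turret for the platformer that fires BP_Bullet from its FiringPoint continuously from BeginPlay.
; UseScatterShot picks either single shots or bursts with random pitch and yaw spread within ScatterRange, each mode re-calling itself after FiringDelay.
; When LookAtPlayer is set, Tick turns the turret body toward the player pawn using only X and Y positions, applied as relative rotation.
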(event `OneShot`
  ; Shoot
  (`|SpawnActorFromClass` "/Game/_Platformer/Blueprints/BP_Bullet.BP_Bullet_C" (`SceneComponent.GetSocketTransform` (`self.FiringPoint`) "None" "RTS_World") "AlwaysSpawn" "MultiplyWithRoot" null null)
  (`KismetSystemLibrary.Delay` (`self.FiringDelay`))
  (`self.OneShot`))

(event `self.ReceiveBeginPlay`
  (if (`self.UseScatterShot`)
    (`self.ScatterShot`)
    (else
      (`self.OneShot`))))

(event `ScatterShot`
  (bind _firingpoint (`self.FiringPoint`))
  (bind _scatterrange (`self.ScatterRange`))
  (bind (_returnvalue_roll _returnvalue_pitch _returnvalue_yaw) (`KismetMathLibrary.BreakRotator` (`SceneComponent.GetSocketRotation` _firingpoint "None")))
  (bind _returnvalue (* _scatterrange -1.0))
  (for _ (range (+ (`self.ScatterBulletNumber`) 1))
    (`|SpawnActorFromClass` "/Game/_Platformer/Blueprints/BP_Bullet.BP_Bullet_C" (`KismetMathLibrary.MakeTransform` (`SceneComponent.GetSocketLocation` _firingpoint "None") (`KismetMathLibrary.MakeRotator` _returnvalue_roll (+ _returnvalue_pitch (`KismetMathLibrary.RandomFloatInRange` _returnvalue _scatterrange)) (+ _returnvalue_yaw (`KismetMathLibrary.RandomFloatInRange` _returnvalue _scatterrange)))) "AlwaysSpawn" "MultiplyWithRoot" null null))
  (`KismetSystemLibrary.Delay` (`self.FiringDelay`))
  (`self.ScatterShot`))

(event `self.ReceiveTick`
  (params (DeltaSeconds :type "Float (single-precision)"))
  (bind (_returnvalue_x _returnvalue_y) (`KismetMathLibrary.BreakVector` (`self.K2_GetActorLocation`)))
  (bind (_returnvalue_x_2 _returnvalue_y_2) (`KismetMathLibrary.BreakVector` (`self.K2_GetActorLocation` (`GameplayStatics.GetPlayerPawn` 0))))
  ; RotateTurret
  (if (`self.LookAtPlayer`)
    (`SceneComponent.K2_SetRelativeRotation` (`self.SM_Turret_Body`) (`KismetMathLibrary.FindLookAtRotation` (`KismetMathLibrary.MakeVector` _returnvalue_x _returnvalue_y) (`KismetMathLibrary.MakeVector` _returnvalue_x_2 _returnvalue_y_2)) false false)))

(fn `UserConstructionScript`)