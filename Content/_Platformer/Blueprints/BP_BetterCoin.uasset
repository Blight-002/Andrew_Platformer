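; BP_BetterCoin is a collectible coin pickup for the platformer.
; When the player pawn overlaps it, the coin plays a ping sound at its mesh location and increments the Coins counter on BP_ThirdPersonCharacter.
; It then destroys itself; BeginPlay, Tick and the construction script add no behavior.
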(event `self.ReceiveActorBeginOverlap`
  (params (OtherActor :type "Actor Object Reference"))
  (bind _returnvalue (`GameplayStatics.GetPlayerPawn` 0))
  (if (== OtherActor _returnvalue)
    (`GameplayStatics.PlaySoundAtLocation` "/Engine/EngineSounds/1kSineTonePing.1kSineTonePing" (`SceneComponent.K2_GetComponentLocation` (`self.SM_Coin`)) (struct) 1.0 1.0 0.0 null null null null)
    (bind _asbp_third_person_character (cast `/Game/_Platformer/Blueprints/BP_ThirdPersonCharacter` _returnvalue))
    (`/Engine/EditorBlueprintResources/StandardMacros.IncrementInt` (`/Game/_Platformer/Blueprints/BP_ThirdPersonCharacter.Coins` _asbp_third_person_character)
      (:`  `
        (`self.K2_DestroyActor`)))))

(fn `UserConstructionScript`
  (`parent.UserConstructionScript`))